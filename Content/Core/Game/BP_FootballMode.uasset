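; Game mode for a two-team football game that assigns players to Red or Blue and manages the ball.
; ChoosePlayerStart records each player's side in a map and alternates it when a PlayerStart with the matching tag is found, otherwise picking a random start.
; SpawnDefaultPawnFor spawns the third-person character with that side.
; RefreshBall, run on the server at BeginPlay, uses a short timer to spawn or teleport the ball above the origin.
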(event Custom|ResetBall
  (Variables|Default|GetBallActor
    (:then
      _)
    (:else
      (bind _returnvalue (Game|SpawnActorfromClass "/Game/Core/Ball/BP_Ball.BP_Ball_C" (Math|Transform|MakeTransform "0, 0, 0" "0, 0, 0" "1.000000,1.000000,1.000000") "Undefined" "MultiplyWithRoot" 0 0))
      (Variables|Default|SetBallActor _returnvalue)))
  (Transformation|SetActorLocation (Variables|Default|GetBallActor) "0.000000,0.000000,500.000000" false true))

(event EventBeginPlay
  (Networking|SwitchHasAuthority
    (:Authority
      (CallFunction|RefreshBall))))

(event EventTick
  (params (DeltaSeconds :type Float%20%28single-precision%29)))

(event EventRefreshBall
  (Utilities|Time|SetTimerbyFunctionName 0 "ResetBall" 2.0))

(fn ConstructionScript)

(fn ChoosePlayerStart
  (params (Player :type Controller%20Object%20Reference))
  (bind _outactors (Actor|GetAllActorsOfClass "/Script/Engine.PlayerStart"))
  (LocalVariables|SetPlayerStartList _outactors)
  (Utilities|Map|Add (Variables|Default|GetPlayers) Player (Variables|Default|GetLastSide))
  (for _array_element (LocalVariables|GetPlayerStartList)
    (if (== (Variables|/Script/Engine.PlayerStart|GetPlayerStartTag _array_element) (Utilities|String|EnumtoString (Variables|Default|GetLastSide)))
      (switch Utilities|FlowControl|Switch|SwitchonEPlayerSide (Variables|Default|GetLastSide)
        (:NewEnumerator0
          (Variables|Default|SetLastSide "NewEnumerator1"))
        (:NewEnumerator1
          (Variables|Default|SetLastSide "NewEnumerator0")))
      (return _array_element)))
  (Development|PrintString "PlayerStart with tag not found")
  (return (.OutItem (Utilities|Array|Random (LocalVariables|GetPlayerStartList)))))

(fn SpawnDefaultPawnfor
  (params (NewPlayer :type Controller%20Object%20Reference) (StartSpot :type Actor%20Object%20Reference))
  (bind _players (Variables|Default|GetPlayers))
  (bind (_value _returnvalue) (Utilities|Map|Find _players NewPlayer))
  (bind _returnvalue_2 (Game|SpawnActorfromClass "/Game/Core/Characters/BP_ThirdPersonCharacter.BP_ThirdPersonCharacter_C" (Transformation|GetActorTransform StartSpot) "Undefined" "MultiplyWithRoot" 0 _value 0))
  (if _returnvalue
    (return _returnvalue_2)))