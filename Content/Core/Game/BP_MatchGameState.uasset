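; BP_MatchGameState is the match game state that keeps a per-side goal tally in the Goals map.
; ScoredGoal increments every side except the one passed in, so that Side is treated as the conceding side.
; Each increment broadcasts OnScoreUpdated with the side and new score.
; After the loop, only the authority asks the game mode to refresh the ball through RefreshBallMessage.
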(event EventBeginPlay)

(event EventTick
  (params (DeltaSeconds :type Float%20%28single-precision%29)))

(event EventScoredGoal
  (params (Side :type EPlayerSide%20Enum :default "NewEnumerator0"))
  (bind _goals (Variables|Default|GetGoals))
  (bind (_keypin _valuepin) (Utilities|Map|ForEachLoop(Map) (Variables|Default|GetGoals))
    (:then
      (if (Utilities|Enum|NotEqual(Enum) _keypin Side)
        (Utilities|Map|Add _goals _keypin (+ _valuepin 1))
        (Default|CallOnScoreUpdated _keypin (.Value (Utilities|Map|Find _goals _keypin)))))
    (:CompletedPin
      (Networking|SwitchHasAuthority
        (:Authority
          (Class|BPIFootballMode|RefreshBall(Message) (Game|GetGameMode)))))))

(fn ConstructionScript)