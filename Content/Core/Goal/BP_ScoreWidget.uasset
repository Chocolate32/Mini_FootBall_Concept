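; BP_ScoreWidget is an actor that displays the match score through a WBP_ScoreWidget in its Widget component.
; On authority it binds to the BP_MatchGameState score-updated event and forwards side and score to UpdateScoreUI.
; Only remote instances create the widget, passing in SwitchSides, and UpdateScoreUI updates it only there.
; The authority instance therefore never creates or updates the display itself.
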(event Custom|OnScoreUpdated_Event
  (params (Side :type EPlayerSide%20Enum :default "NewEnumerator0") (Score :type Integer))
  (CallFunction|UpdateScoreUI Side Score))

(event Custom|UpdateScoreUI
  (params (Side :type EPlayerSide%20Enum :default "NewEnumerator0") (Score :type Integer))
  (Networking|SwitchHasAuthority
    (:Remote
      (bind _scorewidget (Variables|Default|GetScoreWidget)
        (:then
          (Default|OnScoreUpdated _scorewidget Side Score))
        (:else
          (Development|PrintString "Widget is not valid"))))))

(event EventBeginPlay
  (bind _returnvalue (Game|GetGameState))
  (Networking|SwitchHasAuthority
    (:Authority
      (Utilities|IsValid _returnvalue
        (:Is%20Valid
          (bind _asbp_match_game_state (Utilities|Casting|CastToBP_MatchGameState _returnvalue))
          (EventDispatchers|AssignOnScoreUpdated _asbp_match_game_state (delegate Custom|OnScoreUpdated_Event)))))
    (:Remote
      (bind _returnvalue_2 (UserInterface|CreateWidget "/Game/Core/UI/WBP_ScoreWidget.WBP_ScoreWidget_C" 0 (Variables|Default|GetSwitch%20Sides)))
      (UserInterface|SetWidget (Variables|Default|GetWidget) _returnvalue_2)
      (Variables|Default|SetScoreWidget _returnvalue_2))))

(event Collision|EventActorBeginOverlap
  (params (OtherActor :type Actor%20Object%20Reference)))

(event EventTick
  (params (DeltaSeconds :type Float%20%28single-precision%29)))

(fn ConstructionScript)