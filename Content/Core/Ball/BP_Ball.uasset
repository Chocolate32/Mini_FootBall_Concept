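; BP_Ball is a physics-driven ball actor that exposes events for pushing, shooting and slowing it.
; ShootTowards scales a direction by a force and passes it to AddImpulse, which applies it to BallMesh as a mass-independent velocity change.
; SlowVelocity replaces the mesh's linear velocity with its normalized vector, keeping the heading but cutting speed to one unit per second.
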(event Custom|AddImpulse
  (params (Impulse :type Vector))
  (Physics|AddImpulse (Variables|Default|GetBallMesh) Impulse "None" true))

(event EventBeginPlay)

(event Collision|EventActorBeginOverlap
  (params (OtherActor :type Actor%20Object%20Reference)))

(event EventTick
  (params (DeltaSeconds :type Float%20%28single-precision%29)))

(event EventShootTowards
  (params (Direction :type Vector :default "0, 0, 0") (Force :type Float%20%28double-precision%29))
  (CallFunction|AddImpulse (* Direction Force)))

(event EventSlowVelocity
  (bind _returnvalue (Physics|GetPhysicsLinearVelocity (Variables|Default|GetBallMesh) "None"))
  (Physics|SetPhysicsLinearVelocity (Variables|Default|GetBallMesh) (Math|Vector|Normalize _returnvalue) false "None"))

(fn ConstructionScript)